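; MasterWeaponBP is a weapon Blueprint, named as a master class, that provides automatic hitscan fire between StartFire and StopFire.
; A Gate re-enters itself through a short retriggerable delay to repeat shots until StopFire closes it.
; Each shot traces on Visibility from the owner's eye point along the actor's forward vector, then plays a shutter sound and calls PlayMontage.
; Both hit-result branches are empty, so shots apply no effect.
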(event Custom|StartFire
  (bind _returnvalue (Components|GetOwner))
  (bind _outlocation (Actor|GetActorEyesViewPoint _returnvalue))
  (Utilities|FlowControl|Sequence
    (:then_0
      (goto _label Open))
    (:then_1
      (Utilities|FlowControl|Gate true :!label _label
        (:Exit
          (Utilities|FlowControl|Sequence
            (:then_0
              (Utilities|FlowControl|RetriggerableDelay 0.1)
              (goto _label))
            (:then_1
              (bind _returnvalue_2 (Collision|LineTraceByChannel _outlocation (+ _outlocation (* (Transformation|GetActorForwardVector _returnvalue) 1.5e+04)) "TraceTypeQuery1" false 0 "None"))
              (if _returnvalue_2
                _
                (else
                  _))
              (Audio|PlaySound2D "/Engine/VREditor/Sounds/UI/Camera_Shutter.Camera_Shutter" 1.0 1.0 0.0 0 0)
              (Animation|Montage|PlayMontage 0 0))))))))

(event Custom|StopFire
  (bind _returnvalue (Components|GetOwner))
  (bind _outlocation (Actor|GetActorEyesViewPoint _returnvalue))
  (Utilities|FlowControl|Gate true) ; enters at Close
)

(event EventBeginPlay)

(event Collision|EventActorBeginOverlap
  (params (OtherActor :type Actor%20Object%20Reference)))

(event EventTick
  (params (DeltaSeconds :type Float%20%28single-precision%29)))

(fn ConstructionScript)